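; BP_RoomConnectionDoor is a door between rooms that slides along Z when a Character enters its trigger box.
; CanOpen sets whether the door ignores or blocks Pawn and Vehicle collision at BeginPlay, and gates all opening logic.
; Box overlaps play the DoorSlide timeline, reversing it once no Characters remain inside, with an Open flag preventing retriggers.
; A separate OpenDoor function yaws the door 90 degrees but is not called here.
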(event `self.ReceiveBeginPlay`
  (bind _door (`self.Door`))
  (if (`self.CanOpen?`)
    (`PrimitiveComponent.SetCollisionResponseToChannel` _door "ECC_Pawn" "ECR_Ignore")
    (`PrimitiveComponent.SetCollisionResponseToChannel` _door "ECC_Vehicle" "ECR_Ignore")
    (else
      (`PrimitiveComponent.SetCollisionResponseToChannel` _door "ECC_Pawn" "ECR_Block")
      (`PrimitiveComponent.SetCollisionResponseToChannel` _door "ECC_Vehicle" "ECR_Block"))))

(event `self.Box.OnComponentBeginOverlap`
  (params (OverlappedComponent :type "PrimitiveComponent Object Reference") (OtherActor :type "Actor Object Reference") (OtherComp :type "PrimitiveComponent Object Reference") (OtherBodyIndex :type Integer) (bFromSweep :type Boolean) (SweepResult :type "HitResult Structure (by ref)"))
  (if (`self.CanOpen?`)
    (cast `Character` OtherActor)
    (if (not (`self.Open`))
      (set `self.Open` true)
      (bind (_direction _doorslide) (`Timeline|DoorSlide` :!label _label)
        (:`Update`
          (`SceneComponent.K2_SetRelativeLocation` (`self.Door`) (`KismetMathLibrary.MakeVector` 0.0 0.0 _doorslide) false false))))))

(event `self.Box.OnComponentEndOverlap`
  (params (OverlappedComponent :type "PrimitiveComponent Object Reference") (OtherActor :type "Actor Object Reference") (OtherComp :type "PrimitiveComponent Object Reference") (OtherBodyIndex :type Integer))
  (if (`self.CanOpen?`)
    (if (not (> (`KismetArrayLibrary.Array_Length` (`PrimitiveComponent.GetOverlappingActors` (`self.Box`) "/Script/Engine.Character")) 0))
      (cast `Character` OtherActor)
      (if (`self.Open`)
        (set `self.Open` false)
        (goto _label :!via `Reverse`)))))

(fn `OpenDoor`
  (if (`self.CanOpen?`)
    (`SceneComponent.K2_AddRelativeRotation` (`self.Door`) (`KismetMathLibrary.MakeRotator` 0.0 0.0 90.0) false false)))

(fn `UserConstructionScript`)