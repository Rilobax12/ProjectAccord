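; Base enemy character that carries a weapon, shows a health bar and is destroyed when its health runs out.
; BeginPlay spawns the weapon onto the right-hand socket and sets a fixed aim point ahead of the enemy.
; Construction sets walk speed and builds the billboard's dynamic material, sized by max health; RecieveDamage updates its fill.
; An Aiming function handles turn-in-place yaw toward the aim point but is never run.
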(event `self.ReceiveTick`
  (params (DeltaSeconds :type "Float (single-precision)")))

(event `self.ReceiveBeginPlay`
  (bind (_returnvalue_location _returnvalue_rotation _returnvalue_scale) (`KismetMathLibrary.BreakTransform` (`self.GetTransform`)))
  (bind _returnvalue (`|SpawnActorFromClass` (`self.Weapon_Class`) (`KismetMathLibrary.MakeTransform` _returnvalue_location (struct :`Yaw` -90.0) _returnvalue_scale) "Undefined" "OverrideRootScale" null null))
  (bind _output_get (set `self.Weapon` _returnvalue))
  (`self.K2_AttachToComponent` _output_get (`self.Mesh`) "hand_r" "SnapToTarget" "KeepRelative" "SnapToTarget" true)
  (bind _output_get_2 (set `self.AimLocation` (+ (* (`self.GetActorForwardVector`) 200.0) (`self.K2_GetActorLocation`))))
  (set `/Game/Weapons/Weapon_Parent.AimLoc` _output_get_2 (`self.Weapon`)))

(event `Recieve Damage`
  (params (Damage :type "Float (double-precision)"))
  (if (not (<= (`self.Health_Cur`) 0.0))
    (set `self.Health_Cur` (- (`self.Health_Cur`) Damage))
    (`MaterialInstanceDynamic.SetScalarParameterValue` (`self.DynamicHealthBarMaterial`) "PercentFill" (/ (`self.Health_Cur`) (`self.Health_Max`)))
    (if (<= (`self.Health_Cur`) 0.0)
      (set `self.Alive` false)
      (`self.K2_DestroyActor`))))

(fn `Aiming`
  (bind _yaw (.yaw (`KismetMathLibrary.NormalizedDeltaRotator` (`KismetMathLibrary.MakeRotFromX` (`KismetMathLibrary.Normal` (- (`self.AimLocation`) (`self.K2_GetActorLocation`)))) (`self.K2_GetActorRotation`))))
  (bind _returnvalue (`KismetMathLibrary.Abs` _yaw))
  (bind _returnvalue_2 (* _yaw (`self.BaseTurnRate`) (`GameplayStatics.GetWorldDeltaSeconds`)))
  (if (or (`self.TurnRight`) (`self.TurnLeft`) (> (`KismetMathLibrary.VSize` (`self.GetVelocity`)) 1.0))
    (`self.K2_AddActorWorldRotation` (`KismetMathLibrary.MakeRotator` 0.0 0.0 _returnvalue_2))
    (if (not (> _returnvalue 5.0))
      (set `self.TurnRight` false)
      (set `self.TurnLeft` false))
    (elif (> _returnvalue (`self.AimLimit`))
      (if (> _returnvalue_2 0.0)
        (set `self.TurnRight` true)
        (set `self.TurnLeft` false)
        (else
          (set `self.TurnLeft` true)
          (set `self.TurnRight` false))))))

(fn `UserConstructionScript`
  (bind _health_max (`self.Health_Max`))
  (bind _elements (`MaterialBillboardComponent.Elements` (`self.HealthBillboard`)))
  (bind (_output_material _output_distancetoopacitycurve _output_bsizeisinscreenspace _output_basesizex _output_basesizey _output_distancetosizecurve) (break `MaterialSpriteElement` (`|GetArrayItem` _elements)))
  (set `CharacterMovementComponent.MaxWalkSpeed` (`self.MovementSpeed`) (`self.CharacterMovement`))
  (bind _returnvalue (`PrimitiveComponent.CreateDynamicMaterialInstance` (`self.HealthBillboard`) 0 null))
  (bind _output_get (set `self.DynamicHealthBarMaterial` _returnvalue))
  (`MaterialInstanceDynamic.SetScalarParameterValue` _output_get "PercentFill" (/ (`self.Health_Cur`) _health_max))
  (`MaterialInstanceDynamic.SetScalarParameterValue` _output_get "MaxHealth" _health_max)
  (`KismetArrayLibrary.Array_Set` _elements 0 (make `MaterialSpriteElement` _output_material _output_distancetoopacitycurve _output_bsizeisinscreenspace _output_basesizex (* (`self.Health_Max`) 15.0) _output_distancetosizecurve)))