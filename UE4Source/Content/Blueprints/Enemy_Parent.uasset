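; Base enemy character that spots the player through PawnSensing, chases to a preferred range and fires an attached weapon.
; Tick scales walk speed by distance, interpolates the aim point and line-traces to the player to start or stop firing.
; Aiming yaws the body while moving, or turns in place once aim exceeds a limit.
; Damage updates a billboard material health bar; death ragdolls the mesh before delayed destruction.
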(event `self.PawnSensing.OnSeePawn`
  (params (Pawn :type "Pawn Object Reference"))
  (bind _astop_down_character (cast `/Game/Blueprints/TopDownCharacter` Pawn))
  (set `self.Enemy` _astop_down_character)
  (set `self.FoundEnemy` true)
  (if (`KismetMathLibrary.InRange_FloatFloat` (`self.GetDistanceTo` (`self.Enemy`)) (+ (`self.PreferredRange`) 200.0) (`self.MaxFollowRange`))
    (`/Engine/EditorBlueprintResources/StandardMacros.DoOnce` false :!label _label
      (:`Completed`
        (bind _movementresult (`|AIMoveTo` self (0.0 0.0 0.0) (`self.Enemy`) (`self.PreferredRange`))
          (:`then`
            (`KismetSystemLibrary.PrintString` (`|GetEnumeratorNameAsString` _movementresult)))
          (:`OnSuccess`
            (goto _label :!via `Reset`))
          (:`OnFail`
            (set `self.FoundEnemy` false)
            (goto _label :!via `Reset`)))))))

(event `self.ReceiveTick`
  (params (DeltaSeconds :type "Float (single-precision)"))
  (bind _weapon (`self.Weapon`))
  (bind _enemy (`self.Enemy`))
  (bind _preferredrange (`self.PreferredRange`))
  (bind _returnvalue (`KismetMathLibrary.MakeVector` (.x (`self.K2_GetActorLocation`)) (.y (`self.K2_GetActorLocation`)) (+ (.z (`self.K2_GetActorLocation`)) (`self.BaseEyeHeight`))))
  (if (`self.Alive`)
    (`|ExecutionSequence`
      (:`then_0`
        (if (`self.FoundEnemy`)
          (`/Engine/EditorBlueprintResources/StandardMacros.IsValid` _enemy
            (:`Is Valid`
              (set `CharacterMovementComponent.MaxWalkSpeed` (`KismetMathLibrary.MapRangeClamped` (`self.GetDistanceTo` (`self.Enemy`)) _preferredrange (+ _preferredrange 200.0) 100.0 (`self.MovementSpeed`)) (`self.CharacterMovement`))
              (bind _output_get (set `self.AimLocation` (`KismetMathLibrary.VInterpTo` (`self.AimLocation`) (`KismetMathLibrary.MakeVector` (.x (`self.K2_GetActorLocation` _enemy)) (.y (`self.K2_GetActorLocation` _enemy)) (+ (.z (`self.K2_GetActorLocation` _enemy)) (`self.BaseEyeHeight`))) (`GameplayStatics.GetWorldDeltaSeconds`) (`self.AimSpeed`))))
              (set `/Game/Weapons/Weapon_Parent.AimLoc` _output_get (`self.Weapon`))
              (bind (_outhit _returnvalue_2) (`KismetSystemLibrary.LineTraceSingle` _returnvalue (+ (* (`KismetMathLibrary.Normal` (- (`self.K2_GetActorLocation` (`self.Enemy`)) _returnvalue)) (`self.MaxAttackRange`)) _returnvalue) "TraceTypeQuery2"))
              (if _returnvalue_2
                (cast `/Game/Blueprints/TopDownCharacter` (`.HitActor` (`GameplayStatics.BreakHitResult` _outhit))
                  (:`then`
                    (`/Engine/EditorBlueprintResources/StandardMacros.DoOnce` false :!label _label_2
                      (:`Completed`
                        (`/Game/Weapons/Weapon_Parent.Fire` _weapon)
                        (goto _label_3 :!via `Reset`))))
                  (:`CastFailed`
                    _)))
              (`/Engine/EditorBlueprintResources/StandardMacros.DoOnce` false :!label _label_3
                (:`Completed`
                  (`/Game/Weapons/Weapon_Parent.StopFire` _weapon)
                  (goto _label_2 :!via `Reset`)))))
          (else
            (`/Game/Weapons/Weapon_Parent.StopFire` (`self.Weapon`) :!label _label_4))))
      (:`then_1`
        (`self.Aiming`))
      (:`then_2`
        (`SceneComponent.K2_SetWorldLocation` (`self.HealthBillboard`) (+ (`self.K2_GetActorLocation`) (60.0 0.0 100.0)) false false)))
    (else
      (goto _label_4))))

(event `self.ReceiveBeginPlay`
  (bind (_returnvalue_location _returnvalue_rotation _returnvalue_scale) (`KismetMathLibrary.BreakTransform` (`self.GetTransform`)))
  (bind _returnvalue (`|SpawnActorFromClass` (`self.Weapon_Class`) (`KismetMathLibrary.MakeTransform` _returnvalue_location (struct :`Yaw` -90.0) _returnvalue_scale) "Undefined" "OverrideRootScale" null null))
  (bind _output_get (set `self.Weapon` _returnvalue))
  (`self.K2_AttachToComponent` _output_get (`self.Mesh`) "hand_r" "SnapToTarget" "KeepRelative" "SnapToTarget" true)
  (bind _output_get_2 (set `self.AimLocation` (+ (* (`self.GetActorForwardVector`) 200.0) (`self.K2_GetActorLocation`))))
  (set `/Game/Weapons/Weapon_Parent.AimLoc` _output_get_2 (`self.Weapon`)))

(event `Recieve Damage`
  (params (Damage :type "Float (double-precision)"))
  (bind _mesh (`self.Mesh`))
  (if (not (<= (`self.Health_Cur`) 0.0))
    (set `self.Health_Cur` (- (`self.Health_Cur`) Damage))
    (`MaterialInstanceDynamic.SetScalarParameterValue` (`self.DynamicHealthBarMaterial`) "PercentFill" (/ (`self.Health_Cur`) (`self.Health_Max`)))
    (if (<= (`self.Health_Cur`) 0.0)
      (set `self.Alive` false)
      (`PrimitiveComponent.SetCollisionObjectType` _mesh "ECC_PhysicsBody")
      (`PrimitiveComponent.SetCollisionEnabled` _mesh "QueryAndPhysics")
      (`PrimitiveComponent.SetSimulatePhysics` _mesh true)
      (`SceneComponent.SetVisibility` (`self.HealthBillboard`) false false)
      (`KismetSystemLibrary.Delay` 5.0)
      (`self.K2_DestroyActor`)
      (`self.K2_DestroyActor` (`self.Weapon`)))))

(fn `Aiming`
  (bind _yaw (.yaw (`KismetMathLibrary.NormalizedDeltaRotator` (`KismetMathLibrary.MakeRotFromX` (`KismetMathLibrary.Normal` (- (`self.AimLocation`) (`self.K2_GetActorLocation`)))) (`self.K2_GetActorRotation`))))
  (bind _returnvalue (`KismetMathLibrary.Abs` _yaw))
  (bind _returnvalue_2 (* _yaw (`self.BaseTurnRate`) (`GameplayStatics.GetWorldDeltaSeconds`)))
  (if (or (`self.TurnRight`) (`self.TurnLeft`) (> (`KismetMathLibrary.VSize` (`self.GetVelocity`)) 1.0))
    (`self.K2_AddActorWorldRotation` (`KismetMathLibrary.MakeRotator` 0.0 0.0 _returnvalue_2))
    (if (not (> _returnvalue 5.0))
      (set `self.TurnRight` false)
      (set `self.TurnLeft` false))
    (elif (> _returnvalue (`self.AimLimit`))
      (if (> _returnvalue_2 0.0)
        (set `self.TurnRight` true)
        (set `self.TurnLeft` false)
        (else
          (set `self.TurnLeft` true)
          (set `self.TurnRight` false))))))

(fn `UserConstructionScript`
  (bind _health_max (`self.Health_Max`))
  (bind _elements (`MaterialBillboardComponent.Elements` (`self.HealthBillboard`)))
  (bind (_output_material _output_distancetoopacitycurve _output_bsizeisinscreenspace _output_basesizex _output_basesizey _output_distancetosizecurve) (break `MaterialSpriteElement` (`|GetArrayItem` _elements)))
  (set `CharacterMovementComponent.MaxWalkSpeed` (`self.MovementSpeed`) (`self.CharacterMovement`))
  (bind _returnvalue (`PrimitiveComponent.CreateDynamicMaterialInstance` (`self.HealthBillboard`) 0 null))
  (bind _output_get (set `self.DynamicHealthBarMaterial` _returnvalue))
  (`MaterialInstanceDynamic.SetScalarParameterValue` _output_get "PercentFill" (/ (`self.Health_Cur`) _health_max))
  (`MaterialInstanceDynamic.SetScalarParameterValue` _output_get "MaxHealth" _health_max)
  (`KismetArrayLibrary.Array_Set` _elements 0 (make `MaterialSpriteElement` _output_material _output_distancetoopacitycurve _output_bsizeisinscreenspace _output_basesizex (* (`self.Health_Max`) 15.0) _output_distancetosizecurve)))