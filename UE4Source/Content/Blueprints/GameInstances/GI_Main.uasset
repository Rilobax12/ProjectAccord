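; GI_Main is the game instance that handles multiplayer session hosting, joining and the related menus.
; It lazily creates and caches the host and server search widgets before adding them to the viewport.
; LaunchLobby stores the server name, creates a LAN or online session based on the Steam flag, then opens the ALS multiplayer test map as a listen server.
; JoinGame joins a given search result; session failures only print a debug message.
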(event `JoinGame`
  (params (`Session To Join` :type "BlueprintSessionResult Structure"))
  (`JoinSessionCallbackProxy.JoinSession` (`GameplayStatics.GetPlayerController` 0) `Session To Join`
    (:`OnFailure`
      (`KismetSystemLibrary.PrintString` "FAILED"))))

(event `ShowSearchedGames`
  (`/Engine/EditorBlueprintResources/StandardMacros.IsValid` (`self.SearchGame`)
    (:`Is Valid`
      _)
    (:`Is Not Valid`
      (bind _returnvalue (`|CreateWidget` "/Game/UserInterface/Widgets/Widget_SearchGame.Widget_SearchGame_C" (`GameplayStatics.GetPlayerController` 0)))
      (bind _output_get (set `self.SearchGame` _returnvalue))))
  (`UserWidget.AddToViewport` _output_get 0))

(event `HostGameMenu`
  (`/Engine/EditorBlueprintResources/StandardMacros.IsValid` (`self.HostGame`)
    (:`Is Valid`
      _)
    (:`Is Not Valid`
      (bind _returnvalue (`|CreateWidget` "/Game/UserInterface/Widgets/Widget_HostGame01.Widget_HostGame01_C" (`GameplayStatics.GetPlayerController` 0)))
      (bind _output_get (set `self.HostGame` _returnvalue))))
  (`UserWidget.AddToViewport` _output_get 0))

(event `LaunchLobby`
  (params (`Steam?` :type Boolean) (ServerName :type Text))
  (set `self.Name` ServerName)
  (`CreateSessionCallbackProxy.CreateSession` (`GameplayStatics.GetPlayerController` 0) 20 (not `Steam?`)
    (:`OnSuccess`
      (`GameplayStatics.OpenLevel` "ALS_MultiplayerTestMap01" true "listen"))
    (:`OnFailure`
      (`KismetSystemLibrary.PrintString` "FAILED"))))