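; Physics-driven land vehicle Blueprint that maps player input to engine throttle, steering, handbrake and camera rotation, and launches the car forward and upward on BeginPlay.
; A wheel-contact macro, true when any wheel hit is blocking despite its AllWheelsOnGround name, switches steering to air roll and enables air pitch when airborne.
; Tick applies downforce scaled by squared forward speed while grounded, prints engine RPM and feeds it to the audio.
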(event `InputAxis|CameraY`
  (params (AxisValue :type "Float (single-precision)"))
  (`self.AddControllerPitchInput` (* AxisValue -1.0)))

(event `InputAxis|CameraX`
  (params (AxisValue :type "Float (single-precision)"))
  (`self.AddControllerYawInput` AxisValue))

(event `self.ReceiveBeginPlay`
  (`self.InitializeAllSystems`)
  (`PrimitiveComponent.SetPhysicsLinearVelocity` (`self.StaticMesh`) (+ (* (`self.GetActorForwardVector`) 1000.0) (* (0.0 0.0 1.0) 500.0)) false "None"))

(event `InputAxis|Throttle`
  (params (AxisValue :type "Float (single-precision)"))
  (`self.SetEngineThrottle` AxisValue))

(event `InputAxis|Steering`
  (params (AxisValue :type "Float (single-precision)"))
  (`self.AllWheelsOnGround`
    (:`True`
      (`self.SetSteering` AxisValue))
    (:`False`
      (`PrimitiveComponent.AddTorqueInDegrees` (`self.StaticMesh`) (* (`SceneComponent.GetForwardVector` (`self.StaticMesh`)) (* AxisValue (`self.AirRollRate`) -1.0)) "None" true))))

(event `InputAxis|Pitch`
  (params (AxisValue :type "Float (single-precision)"))
  (`self.AllWheelsOnGround`
    (:`False`
      (`PrimitiveComponent.AddTorqueInDegrees` (`self.StaticMesh`) (* (`SceneComponent.GetRightVector` (`self.StaticMesh`)) (* AxisValue (`self.AirRollRate`) 1.0)) "None" true))))

(event `self.ReceiveTick`
  (params (DeltaSeconds :type "Float (single-precision)"))
  (bind _rpm (`LandVehicle_EngineComponent.RPM` (`self.LandVehicle_Engine`)))
  (`self.Downforce`)
  (`KismetSystemLibrary.PrintString` (`KismetStringLibrary.Conv_DoubleToString` _rpm) true true (struct :`G` 0.66 :`B` 1.0 :`A` 1.0) DeltaSeconds)
  (`AudioComponent.SetFloatParameter` (`self.Audio`) "RPM" _rpm))

(event `InputAction|Handbrake`
  (params (Key :type "Key Structure"))
  (:`Pressed`
    (`self.SetHandbrake` true))
  (:`Released`
    (`self.SetHandbrake` false)))

(fn `Downforce`
  (bind _staticmesh (`self.StaticMesh`))
  (`self.AllWheelsOnGround`
    (:`True`
      (`PrimitiveComponent.AddForce` (`self.StaticMesh`) (* (`SceneComponent.GetUpVector` _staticmesh) (* (`KismetMathLibrary.VSizeSquared` (`KismetMathLibrary.ProjectVectorOnToVector` (`self.GetVelocity`) (`SceneComponent.GetForwardVector` _staticmesh))) (`self.DownforceCoef`) -1.0)) "None" false))))

(fn `UserConstructionScript`)