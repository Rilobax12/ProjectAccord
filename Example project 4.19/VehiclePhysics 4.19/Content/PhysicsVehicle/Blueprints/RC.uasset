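; RC is a player-controlled physics vehicle Blueprint that serves as a thin input layer over vehicle functions defined outside this graph.
; BeginPlay initializes all vehicle systems, then throttle and steering axes and the pressed or released handbrake action pass straight to their setters.
; Camera axes drive controller yaw and pitch, with pitch inverted.
; The construction script is empty.
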(event `InputAxis|Camera Y`
  (params (AxisValue :type "Float (single-precision)"))
  (`self.AddControllerPitchInput` (* AxisValue -1.0)))

(event `InputAxis|Camera X`
  (params (AxisValue :type "Float (single-precision)"))
  (`self.AddControllerYawInput` AxisValue))

(event `self.ReceiveBeginPlay`
  (`self.InitializeAllSystems`))

(event `InputAxis|Throttle`
  (params (AxisValue :type "Float (single-precision)"))
  (`self.SetEngineThrottle` AxisValue))

(event `InputAxis|Steering`
  (params (AxisValue :type "Float (single-precision)"))
  (`self.SetSteering` AxisValue))

(event `InputAction|Handbrake`
  (params (Key :type "Key Structure" :default "AnyKey"))
  (:`Pressed`
    (`self.SetHandbrake` true))
  (:`Released`
    (`self.SetHandbrake` false)))

(fn `UserConstructionScript`)