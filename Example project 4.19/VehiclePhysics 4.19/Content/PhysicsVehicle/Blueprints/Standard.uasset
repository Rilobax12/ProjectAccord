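; Standard is a player-controlled physics vehicle that forwards input to its engine, steering and handbrake functions.
; Throttle and steering axes pass straight through, the handbrake follows press and release, and camera axes drive controller yaw and inverted pitch.
; On BeginPlay it initializes all vehicle systems, then launches the static mesh forward and upward by setting its physics linear velocity.
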(event `InputAxis|Camera Y`
  (params (AxisValue :type "Float (single-precision)"))
  (`self.AddControllerPitchInput` (* AxisValue -1.0)))

(event `InputAxis|Camera X`
  (params (AxisValue :type "Float (single-precision)"))
  (`self.AddControllerYawInput` AxisValue))

(event `self.ReceiveBeginPlay`
  (`self.InitializeAllSystems`)
  (`PrimitiveComponent.SetPhysicsLinearVelocity` (`self.StaticMesh`) (+ (* (`self.GetActorForwardVector`) 1000.0) (* (0.0 0.0 1.0) 500.0)) false "None"))

(event `InputAxis|Throttle`
  (params (AxisValue :type "Float (single-precision)"))
  (`self.SetEngineThrottle` AxisValue))

(event `InputAxis|Steering`
  (params (AxisValue :type "Float (single-precision)"))
  (`self.SetSteering` AxisValue))

(event `InputAction|Handbrake`
  (params (Key :type "Key Structure"))
  (:`Pressed`
    (`self.SetHandbrake` true))
  (:`Released`
    (`self.SetHandbrake` false)))

(fn `UserConstructionScript`)